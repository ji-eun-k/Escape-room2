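; BP_password is a trigger actor for a password puzzle that fires an answer-is-right event when solved.
; Entering its Box enables input and shows a prompt widget; releasing F then opens the password widget in UI-only mouse mode.
; The widget reports input back to the actor, which on a correct answer plays a sound, disables the digit buttons, then after a short delay closes the UI and destroys itself.
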(event OnComponentBeginOverlap(Box)
  (params (OverlappedComponent :type Primitive%20Component%20Object%20Reference) (OtherActor :type Actor%20Object%20Reference) (OtherComp :type Primitive%20Component%20Object%20Reference) (OtherBodyIndex :type Integer) (bFromSweep :type Boolean) (SweepResult :type Hit%20Result%20Structure%20%28by%20ref%29))
  (Input|EnableInput (Game|GetPlayerController 0))
  (UserInterface|Viewport|AddtoViewport (Variables|Default|GetpwFUI) 0)
  (Variables|Default|SetIsCollision (not (Variables|Default|GetIsCollision))))

(event OnComponentEndOverlap(Box)
  (params (OverlappedComponent :type Primitive%20Component%20Object%20Reference) (OtherActor :type Actor%20Object%20Reference) (OtherComp :type Primitive%20Component%20Object%20Reference) (OtherBodyIndex :type Integer))
  (Input|DisableInput (Game|GetPlayerController 0))
  (Widget|RemovefromParent (Variables|Default|GetpwFUI))
  (Variables|Default|SetIsCollision (not (Variables|Default|GetIsCollision))))

(event Custom|OnUserInput
  (params (userInput :type Integer))
  (if (== userInput (Variables|Default|GetCorrectAnswer))
    (Utilities|FlowControl|Sequence
      (:then_0
        (Audio|PlaySound2D "/Game/School/sounds/tvClickSound.tvClickSound" 1.0 1.0 0.0 0 0))
      (:then_1
        (Widget|SetIsEnabled (Variables|/Game/School/UI/PasswordUI.PasswordUI_C|GetUpButton1 (Variables|Default|GetpwUI)) false))
      (:then_2
        (Utilities|FlowControl|Delay 1.5)
        (Default|CloseUI (Variables|Default|GetpwUI))
        (Default|CallOnAnswerIsRight)
        (Actor|DestroyActor)))))

(event EventBeginPlay
  (Utilities|FlowControl|Sequence
    (:then_0
      (bind _returnvalue (UserInterface|CreateWidget "/Game/School/UI/PasswordUI.PasswordUI_C"))
      (Variables|Default|SetpwUI _returnvalue))
    (:then_1
      (bind _returnvalue_2 (UserInterface|CreateWidget "/Game/School/UI/PasswordFUI.PasswordFUI_C"))
      (Variables|Default|SetpwFUI _returnvalue_2))
    (:then_2
      (EventDispatchers|BindEventtoOnUserInput (Variables|Default|GetpwUI) (delegate Custom|OnUserInput)))))

(event Collision|EventActorBeginOverlap
  (params (OtherActor :type Actor%20Object%20Reference)))

(event EventTick
  (params (DeltaSeconds :type Float%20%28single-precision%29)))

(event Input|KeyboardEvents|F
  (params (Key :type Key%20Structure :default "None"))
  (bind _returnvalue (Game|GetPlayerController 0))
  (:Released
    (if (Variables|Default|GetIsCollision)
      (UserInterface|Viewport|AddtoViewport (Variables|Default|GetpwUI) 0)
      (Input|SetInputModeUIOnly _returnvalue 0 "DoNotLock")
      (Variables|/Script/Engine.PlayerController|SetbShowMouseCursor _returnvalue true))))

(fn ConstructionScript)